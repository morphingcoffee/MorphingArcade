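; Base interactable Blueprint that shows a prompt widget while focused and provides interact, focus, drop and fire events.
; BeginPlay writes the Action and Name variables into the W_InteractablePrompt hosted by the InteractionTooltipWidget component.
; The construction script hides the tooltip, and the focus events toggle its visibility.
; Interact, drop and fire only print debug strings with the item's name.
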(event EventBeginPlay
  ;[1 1 1] BeginPlay - Populate Tooltip Text
  (bind _asw_interactable_prompt (Utilities|Casting|CastToW_InteractablePrompt (UserInterface|GetUserWidgetObject (Variables|Default|GetInteractionTooltipWidget))))
  (Variables|Default|SetAs%20W%20Interactable%20Prompt _asw_interactable_prompt)
  (Rendering|Components|TextRender|SetText (Variables|/Game/UI/Widgets/W_InteractablePrompt.W_InteractablePrompt_C|GetActionTitle _asw_interactable_prompt) (Utilities|Text|ToText(String) (Variables|Default|GetAction)))
  (Rendering|Components|TextRender|SetText (Variables|/Game/UI/Widgets/W_InteractablePrompt.W_InteractablePrompt_C|GetItemTitle _asw_interactable_prompt) (Utilities|Text|ToText(String) (Variables|Default|GetName))))

(event EventOnFocus
  ;[1 1 1] On Focus / On Focus Lost
  (Rendering|SetVisibility (Variables|Default|GetInteractionTooltipWidget) true false)
  (Development|PrintString (Utilities|String|Append "On Focus: " (Variables|Default|GetName))))

(event EventOnFocusLost
  ;[1 1 1] On Focus / On Focus Lost
  (Rendering|SetVisibility (Variables|Default|GetInteractionTooltipWidget) false false)
  (Development|PrintString (Utilities|String|Append "On Focus Lost: " (Variables|Default|GetName))))

(event EventOnInteract
  ;[1 1 1] Interact Event
  (Development|PrintString (Utilities|String|Append "Interacted with: " (Variables|Default|GetName))))

(event EventOnFire
  ;[1 1 1] Fire Interaction
  (Development|PrintString (Utilities|String|Append "On Fire: " (Variables|Default|GetName))))

(event EventOnDrop
  ;[1 1 1] Drop Interaction
  (Development|PrintString (Utilities|String|Append "On Drop: " (Variables|Default|GetName))))

(fn ConstructionScript
  (Rendering|SetVisibility (Variables|Default|GetInteractionTooltipWidget) false false))